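; Demo Game Instance that holds saved stats, attributes and leveling data in memory, keyed by save name.
; On Init it copies all three maps from the stats save object.
; Save events add entries to these maps, and matching Load functions return the data with a found flag.
; The save events only update the in-memory maps and do not write back to the save object.
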(event EventSaveStats
  (params (SaveName :type String) (Data :type S%20Stats%20Save%20Data%20Structure))
  (Utilities|Map|Add (Variables|Default|GetSavedStatsData) SaveName Data))

(event EventSaveAttributes
  (params (SaveName :type String) (Data :type S%20Attributes%20Save%20Data%20Structure))
  (Utilities|Map|Add (Variables|Default|GetSavedAttributesData) SaveName Data))

(event EventSaveLeveling
  (params (SaveName :type String) (Data :type S%20Leveling%20Save%20Data%20Structure))
  (Utilities|Map|Add (Variables|Default|GetSavedLevelingData) SaveName Data))

(event EventInit
  (CallFunction|DumpFileDiskData))

(fn DumpFileDiskData
  (bind _output_get (LocalVariables|SetLocalSaveObject (CallFunction|GetStatsSaveObject)))
  (Variables|Default|SetSavedStatsData (Variables|/Game/OpenRPG_Stats/Blueprints/BP_StatsSaveObject.BP_StatsSaveObject_C|GetSavedStatsData _output_get))
  (Variables|Default|SetSavedAttributesData (Variables|/Game/OpenRPG_Stats/Blueprints/BP_StatsSaveObject.BP_StatsSaveObject_C|GetSavedAttributesData (LocalVariables|GetLocalSaveObject)))
  (Variables|Default|SetSavedLevelingData (Variables|/Game/OpenRPG_Stats/Blueprints/BP_StatsSaveObject.BP_StatsSaveObject_C|GetSavedLevelingData (LocalVariables|GetLocalSaveObject)))
  (return))

(fn LoadAttributes
  (params (SaveName :type String))
  (bind _savedattributesdata (Variables|Default|GetSavedAttributesData))
  (bind (_value _returnvalue) (Utilities|Map|Find _savedattributesdata SaveName))
  (return _returnvalue _value))

(fn LoadLeveling
  (params (SaveName :type String))
  (bind _savedlevelingdata (Variables|Default|GetSavedLevelingData))
  (bind (_value _returnvalue) (Utilities|Map|Find _savedlevelingdata SaveName))
  (return _returnvalue _value))

(fn LoadStats
  (params (SaveName :type String))
  (bind _savedstatsdata (Variables|Default|GetSavedStatsData))
  (bind (_value _returnvalue) (Utilities|Map|Find _savedstatsdata SaveName))
  (return _returnvalue _value))