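; BP_DemoEnemy is a selectable demo enemy whose stats component drives a shared enemy widget owned by the player's main UI.
; BeginPlay stores its location, retries until the player's widget exists, then registers it, initializes stats and applies permanent health regeneration.
; Selection events toggle widget visibility and notify the component, with name and level refreshed on select.
; Regeneration ticks add their value to a stat's current value.
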(event OnEffectTick(BP_DemoEnemyStats)
  (params (Effect :type Name :default "None") (Value :type Float%20%28single-precision%29) (Permanent? :type Boolean) (RemainingTicks :type Integer))
  (switch name Effect
    (:HealthRegeneration
      (Default|ModifyStatCurrentValue (Variables|Default|GetBP_DemoEnemyStats) "NewEnumerator0" Value))))

(event Custom|OnSelected
  (Default|UpdateEnemyName (Variables|Default|GetWidget) (Variables|Default|GetEnemyName))
  (Default|UpdateEnemyLevel (Variables|Default|GetWidget) (Variables|Default|GetEnemyLevel))
  (Default|OnOwnerSelected (Variables|Default|GetBP_DemoEnemyStats))
  (Widget|SetVisibility (Variables|Default|GetWidget) "Visible"))

(event Custom|OnSelectionRemoved
  (Default|OnOwnerSelectionRemoved (Variables|Default|GetBP_DemoEnemyStats))
  (Widget|SetVisibility (Variables|Default|GetWidget) "Hidden"))

(event EventBeginPlay
  (bind _bp_demoenemystats (Variables|Default|GetBP_DemoEnemyStats))
  (Utilities|FlowControl|Delay 0.2)
  (Variables|Default|SetStartingLocation (Transformation|GetActorLocation))
  (bind _asbp_demo_character (Utilities|Casting|CastToBP_DemoCharacter (Game|GetPlayerCharacter 0) :!label _label)
    (:then
      (Utilities|IsValid (Variables|/Game/Stats_Demo/Blueprints/BP_DemoCharacter.BP_DemoCharacter_C|GetWB_MainWidget _asbp_demo_character)
        (:Is%20Valid
          (bind _output_get (Variables|Default|SetWidget (Variables|/Game/Stats_Demo/Widgets/WB_DemoMain.WB_DemoMain_C|GetWB_DemoEnemy (Variables|/Game/Stats_Demo/Blueprints/BP_DemoCharacter.BP_DemoCharacter_C|GetWB_MainWidget _asbp_demo_character))))
          (Default|AddCustomWidgets (Variables|Default|GetBP_DemoEnemyStats) (Utilities|Array|MakeArray _output_get))
          (Default|Initialize _bp_demoenemystats)
          (Default|ApplyEffect _bp_demoenemystats "HealthRegeneration" (Utilities|Struct|Makes_Effect 2e+01 2000 1.0 true)))
        (:Is%20Not%20Valid
          (Utilities|FlowControl|Delay 0.1 :!label _label_2)
          (goto _label))))
    (:CastFailed
      (goto _label_2))))

(fn ConstructionScript)