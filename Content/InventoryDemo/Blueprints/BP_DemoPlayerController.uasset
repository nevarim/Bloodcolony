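; Player controller for the inventory demo that owns the main UI and toggles the inventory and equipment windows.
; On BeginPlay it creates WB_DemoMain, adds it to the viewport and enables game-and-UI input with a visible cursor.
; The I and J keys toggle inventory and equipment visibility.
; Getter functions expose the windows and slot containers, selected by container type for player inventory, storage or shop, returning empty if the main widget is invalid.
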(event EventBeginPlay
  ;[0.04365 0.474 1] At beginplay the main widget is created (if not already created by GetContainerWidget or GetEquipmentContainerWidget) and set some settings properly to be able to interact with the UI
  (bind _returnvalue (UserInterface|CreateWidget "/Game/InventoryDemo/Widgets/WB_DemoMain.WB_DemoMain_C"))
  (Variables|Default|SetWB_Main _returnvalue)
  (Input|SetInputModeGameandUI self (Variables|Default|GetWB_Main) "DoNotLock" false)
  (Variables|Default|SetbShowMouseCursor true)
  (UserInterface|Viewport|AddtoViewport (Variables|Default|GetWB_Main) 0))

(event Input|KeyboardEvents|J
  (params (Key :type Key%20Structure))
  (bind _playerequipment (CallFunction|GetPlayerEquipment))
  (bind _mainequipmentwidget (Variables|/Game/OpenRPG_Equipment/Blueprints/Components/BPC_Equipment.BPC_Equipment_C|GetMainEquipmentWidget _playerequipment))
  ;[0.2601 1 0.3249] Show/Hide the inventory and equipment window
  (:Pressed
    (Widget|SetVisibility _mainequipmentwidget (select (Widget|IsVisible _mainequipmentwidget) "Hidden" "Visible"))))

(event Input|KeyboardEvents|I
  (params (Key :type Key%20Structure))
  (bind _playerinventory (CallFunction|GetPlayerInventory))
  ;[0.2601 1 0.3249] Show/Hide the inventory and equipment window
  (:Pressed
    (Default|ChangeWidgetVisibility _playerinventory (not (Widget|IsVisible (Variables|/Game/OpenRPG_Inventory/Blueprints/Components/BPC_ItemsContainer.BPC_ItemsContainer_C|GetMainContainerWidget _playerinventory))))))

(fn ConstructionScript)

(fn GetEquipmentContainerWidget
  (Utilities|IsValid (Variables|Default|GetWB_Main)
    (:Is%20Valid
      (return (Variables|/Game/InventoryDemo/Widgets/WB_DemoEquipmentWindow.WB_DemoEquipmentWindow_C|GetWB_EquipmentSlotsContainer (Variables|/Game/InventoryDemo/Widgets/WB_DemoMain.WB_DemoMain_C|GetWB_DemoEquipmentWindow (Variables|Default|GetWB_Main)))))
    (:Is%20Not%20Valid
      (return 0))))

(fn GetItemsContainerWidget
  (params (Container :type e_ContainerType%20Enum :default "NewEnumerator0"))
  (bind _wb_main (Variables|Default|GetWB_Main))
  (LocalVariables|SetLocalContainer Container)
  (Utilities|IsValid (Variables|Default|GetWB_Main)
    (:Is%20Valid
      (return (Utilities|Select :Index (LocalVariables|GetLocalContainer) :NewEnumerator0 (Variables|/Game/InventoryDemo/Widgets/WB_DemoInventoryWindow.WB_DemoInventoryWindow_C|GetWB_ItemsContainerGrid (Variables|/Game/InventoryDemo/Widgets/WB_DemoMain.WB_DemoMain_C|GetWB_DemoInventoryWindow _wb_main)) :NewEnumerator1 (Variables|/Game/InventoryDemo/Widgets/WB_DemoWindow.WB_DemoWindow_C|GetWB_ItemsContainerGrid (Variables|/Game/InventoryDemo/Widgets/WB_DemoMain.WB_DemoMain_C|GetWB_DemoStorageWindow _wb_main)) :NewEnumerator2 (Variables|/Game/InventoryDemo/Widgets/WB_DemoWindow.WB_DemoWindow_C|GetWB_ItemsContainerGrid (Variables|/Game/InventoryDemo/Widgets/WB_DemoMain.WB_DemoMain_C|GetWB_DemoShopWindow _wb_main)))))
    (:Is%20Not%20Valid
      (return 0))))

(fn GetMainEquipmentWidget
  (Utilities|IsValid (Variables|Default|GetWB_Main)
    (:Is%20Valid
      (return (Variables|/Game/InventoryDemo/Widgets/WB_DemoMain.WB_DemoMain_C|GetWB_DemoEquipmentWindow (Variables|Default|GetWB_Main))))
    (:Is%20Not%20Valid
      (return 0))))

(fn GetMainItemsContainerWidget
  (params (Container :type e_ContainerType%20Enum :default "NewEnumerator0"))
  (bind _wb_main (Variables|Default|GetWB_Main))
  (LocalVariables|SetLocalContainer Container)
  (Utilities|IsValid _wb_main
    (:Is%20Valid
      (return (Utilities|Select :Index (LocalVariables|GetLocalContainer) :NewEnumerator0 (Variables|/Game/InventoryDemo/Widgets/WB_DemoMain.WB_DemoMain_C|GetWB_DemoInventoryWindow _wb_main) :NewEnumerator1 (Variables|/Game/InventoryDemo/Widgets/WB_DemoMain.WB_DemoMain_C|GetWB_DemoStorageWindow _wb_main) :NewEnumerator2 (Variables|/Game/InventoryDemo/Widgets/WB_DemoMain.WB_DemoMain_C|GetWB_DemoShopWindow _wb_main))))
    (:Is%20Not%20Valid
      (return 0))))