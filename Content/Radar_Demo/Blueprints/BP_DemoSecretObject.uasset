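; BP_DemoSecretObject is a radar demo object that highlights itself on the radar of nearby actors.
; When its collision sphere begins overlapping an actor that has a BPC_Radar component, it adds itself as a highlight actor, and removes itself when the overlap ends.
; The construction script sizes the sphere from the ColisionRadius variable.
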(event OnComponentBeginOverlap(Colision)
  (params (OverlappedComponent :type Primitive%20Component%20Object%20Reference) (OtherActor :type Actor%20Object%20Reference) (OtherComp :type Primitive%20Component%20Object%20Reference) (OtherBodyIndex :type Integer) (bFromSweep :type Boolean) (SweepResult :type Hit%20Result%20Structure%20%28by%20ref%29))
  (bind _returnvalue (Actor|GetComponentbyClass OtherActor "/Game/OpenRPG_RadarSystem/Blueprints/BPC_Radar.BPC_Radar_C"))
  ;[0.4125 1 0.06453] When something overlaps we check if its the player, if so we add this instance to the radar
  (Utilities|IsValid _returnvalue
    (:Is%20Valid
      (Default|AddHighLightActor _returnvalue self))))

(event OnComponentEndOverlap(Colision)
  (params (OverlappedComponent :type Primitive%20Component%20Object%20Reference) (OtherActor :type Actor%20Object%20Reference) (OtherComp :type Primitive%20Component%20Object%20Reference) (OtherBodyIndex :type Integer))
  (bind _returnvalue (Actor|GetComponentbyClass OtherActor "/Game/OpenRPG_RadarSystem/Blueprints/BPC_Radar.BPC_Radar_C"))
  ;[0.4125 1 0.06453] Reverse operation
  (Utilities|IsValid _returnvalue
    (:Is%20Valid
      (Default|RemoveHighLightActor _returnvalue self))))

(fn ConstructionScript
  (Components|Sphere|SetSphereRadius (Variables|Default|GetColision) (Variables|Default|GetColisionRadius) true))