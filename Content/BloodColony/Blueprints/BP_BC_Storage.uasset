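; BP_BC_Storage is a placeable storage container that players with a BPC_PlayerInventory can open.
; An overlap sphere sized by InteractRadius registers it as the player's NearbyStorage and shows a "Storage" prompt widget.
; Interacting toggles the BPCStorage container widget, reloading its saved contents by StorageSaveName before showing it.
; Leaving the sphere clears the reference, saves the container to disk and closes the widget.
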(event OnComponentBeginOverlap(InteractColision)
  (params (OverlappedComponent :type Primitive%20Component%20Object%20Reference) (OtherActor :type Actor%20Object%20Reference) (OtherComp :type Primitive%20Component%20Object%20Reference) (OtherBodyIndex :type Integer) (bFromSweep :type Boolean) (SweepResult :type Hit%20Result%20Structure%20%28by%20ref%29))
  (bind _returnvalue (Actor|GetComponentbyClass OtherActor "/Game/OpenRPG_Inventory/Blueprints/Components/BPC_PlayerInventory.BPC_PlayerInventory_C"))
  (Utilities|IsValid _returnvalue
    (:Is%20Valid
      (Variables|/Game/OpenRPG_Inventory/Blueprints/Components/BPC_PlayerInventory.BPC_PlayerInventory_C|SetNearbyStorage _returnvalue self)
      (Rendering|SetVisibility (Variables|Default|GetInteractWidget) true false))))

(event OnComponentEndOverlap(InteractColision)
  (params (OverlappedComponent :type Primitive%20Component%20Object%20Reference) (OtherActor :type Actor%20Object%20Reference) (OtherComp :type Primitive%20Component%20Object%20Reference) (OtherBodyIndex :type Integer))
  (bind _returnvalue (Actor|GetComponentbyClass OtherActor "/Game/OpenRPG_Inventory/Blueprints/Components/BPC_PlayerInventory.BPC_PlayerInventory_C"))
  (Utilities|IsValid _returnvalue
    (:Is%20Valid
      (Variables|/Game/OpenRPG_Inventory/Blueprints/Components/BPC_PlayerInventory.BPC_PlayerInventory_C|SetNearbyStorage _returnvalue 0)
      (Rendering|SetVisibility (Variables|Default|GetInteractWidget) false false)
      (Default|SaveContainer (Variables|Default|GetBPC_Storage) (Variables|Default|GetStorageSaveName) true)
      (Default|ChangeWidgetVisibility (Variables|Default|GetBPC_Storage) false))))

(event EventBeginPlay
  (bind _aswb_demo_interact_text (Utilities|Casting|CastToWB_DemoInteractText (UserInterface|GetUserWidgetObject (Variables|Default|GetInteractWidget)))) ; Get the widget from the component
  (bind _output_get (Variables|Default|SetWB_InteractText _aswb_demo_interact_text))
  (Default|Initialize _output_get "Storage" "O")
  (Rendering|SetVisibility (Variables|Default|GetInteractWidget) false false)
  (Default|LoadContainer (Variables|Default|GetBPC_Storage) (Variables|Default|GetStorageSaveName))
  (Default|Initialize (Variables|Default|GetBPC_Storage)))

(event EventOnInteract
  (params (Actor :type Actor%20Object%20Reference))
  (Utilities|IsValid (Actor|GetComponentbyClass Actor "/Game/OpenRPG_Inventory/Blueprints/Components/BPC_PlayerInventory.BPC_PlayerInventory_C") ; Is a player?
    (:Is%20Valid
      (if (Widget|IsVisible (Variables|/Game/OpenRPG_Inventory/Blueprints/Components/BPC_ItemsContainer.BPC_ItemsContainer_C|GetMainContainerWidget (Variables|Default|GetBPC_Storage)))
        (Default|ChangeWidgetVisibility (Variables|Default|GetBPC_Storage) false)
        (else
          (Default|LoadContainer (Variables|Default|GetBPC_Storage) (Variables|Default|GetStorageSaveName))
          (Default|UpdateContainerWidget (Variables|Default|GetBPC_Storage))
          (Default|ChangeWidgetVisibility (Variables|Default|GetBPC_Storage) true))))))

(fn ConstructionScript
  (Components|Sphere|SetSphereRadius (Variables|Default|GetInteractColision) (Variables|Default|GetInteractRadius) true)
  (Components|StaticMesh|SetStaticMesh (Variables|Default|GetMesh) (Variables|Default|GetStorageMesh)))