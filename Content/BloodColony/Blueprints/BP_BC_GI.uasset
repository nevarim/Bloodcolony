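; Game instance that caches container, player inventory and equipment data in name-keyed maps and persists it to disk.
; On Init it loads separate inventory and equipment save slots, creating save objects if none exist.
; Components store and fetch entries through save and load calls.
; Saving to disk writes player inventory, equipment and only containers flagged disk-saveable; other containers are added just to the in-memory map.
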(event EventSaveEquipment
  (params (SaveName :type String) (Data :type S%20Equipment%20Save%20Data%20Structure))
  ;[1 0.4248 0.1197] Iteraction with the components to store data
  (Utilities|Map|Add (Variables|Equipment|GetSavedEquipment) SaveName Data))

(event EventSaveContainer
  (params (SaveName :type String) (DiskSaveable? :type Boolean) (Data :type S%20Container%20Save%20Data%20Structure))
  ;[1 0.4248 0.1197] Iteraction with the components to store data
  (Utilities|Map|Add (Variables|Inventory|GetSavedContainers) SaveName Data)
  (Utilities|Map|Add (Variables|Inventory|GetDiskSaveableContainers) SaveName DiskSaveable?))

(event EventSavePlayerInventoryData
  (params (SaveName :type String) (Data :type S%20Player%20Inventory%20Save%20Data%20Structure))
  ;[1 0.4248 0.1197] Iteraction with the components to store data
  (Utilities|Map|Add (Variables|Inventory|GetSavedPlayerData) SaveName Data))

(event EventInit
  ;[1 0.08333 0.08333] Load some possible data from disk
  (CallFunction|LoadDiskData))

(event EventLoadDatafromDisk
  ;[0.1051 0.2513 1] Interaction with the .sav file on disk
  (CallFunction|LoadDiskData))

(event EventSaveDatatoDisk
  ;[0.1051 0.2513 1] Interaction with the .sav file on disk
  (CallFunction|SaveGameData))

(fn LoadDiskSlot
  (params (SlotName :type String) (SaveClass :type Save%20Game%20Class%20Reference))
  (LocalVariables|SetLocalSlotName SlotName)
  (LocalVariables|SetLocalSaveClass SaveClass)
  (bind _returnvalue (SaveGame|DoesSaveGameExist (LocalVariables|GetLocalSlotName)))
  (if _returnvalue
    (bind _returnvalue_2 (SaveGame|LoadGamefromSlot (LocalVariables|GetLocalSlotName)))
    (return _returnvalue_2)
    (else
      (bind _returnvalue_3 (SaveGame|CreateSaveGameObject (LocalVariables|GetLocalSaveClass)))
      (return _returnvalue_3))))

(fn LoadDiskData
  (bind _asinventory_save (Utilities|Casting|CastToInventorySave (CallFunction|LoadDiskSlot (Variables|Inventory|GetInventorySystemSlotName) (Variables|Inventory|GetInventorySystemSaveClass)))
    (:then
      (bind _output_get (Variables|Inventory|SetInventorySystemSaveObject _asinventory_save))
      (Variables|Inventory|SetSavedContainers (Variables|/Game/OpenRPG_Inventory/Blueprints/Save/InventorySave.InventorySave_C|GetSavedContainers _output_get))
      (Variables|Inventory|SetSavedPlayerData (Variables|/Game/OpenRPG_Inventory/Blueprints/Save/InventorySave.InventorySave_C|GetSavedPlayerData (Variables|Inventory|GetInventorySystemSaveObject)))
      (bind _asequipment_save (Utilities|Casting|CastToEquipmentSave (CallFunction|LoadDiskSlot (Variables|Equipment|GetEquipmentSystemSlotName) (Variables|Equipment|GetEquipmentSystemSaveClass)))
        (:then
          (bind _output_get_2 (Variables|Equipment|SetEquipmentSystemSaveObject _asequipment_save))
          (Variables|Equipment|SetSavedEquipment (Variables|/Game/OpenRPG_Equipment/Blueprints/Saving/EquipmentSave.EquipmentSave_C|GetSavedEquipment _output_get_2))
          (return))
        (:CastFailed
          (return))))
    (:CastFailed
      (return))))

(fn SaveGameData
  (bind _keys (Utilities|Map|Keys (Variables|Inventory|GetDiskSaveableContainers)))
  (for _array_element _keys
    (bind _output_get (LocalVariables|SetLocalSaveName _array_element))
    (if (.Value (Utilities|Map|Find (Variables|Inventory|GetDiskSaveableContainers) _output_get))
      (Utilities|Map|Add (Variables|/Game/OpenRPG_Inventory/Blueprints/Save/InventorySave.InventorySave_C|GetSavedContainers (Variables|Inventory|GetInventorySystemSaveObject)) (LocalVariables|GetLocalSaveName) (.Value (Utilities|Map|Find (Variables|Inventory|GetSavedContainers) (LocalVariables|GetLocalSaveName))))))
  (Variables|/Game/OpenRPG_Inventory/Blueprints/Save/InventorySave.InventorySave_C|SetSavedPlayerData (Variables|Inventory|GetInventorySystemSaveObject) (Variables|Inventory|GetSavedPlayerData))
  (SaveGame|SaveGametoSlot (Variables|Inventory|GetInventorySystemSaveObject) (Variables|Inventory|GetInventorySystemSlotName))
  (Variables|/Game/OpenRPG_Equipment/Blueprints/Saving/EquipmentSave.EquipmentSave_C|SetSavedEquipment (Variables|Equipment|GetEquipmentSystemSaveObject) (Variables|Equipment|GetSavedEquipment))
  (SaveGame|SaveGametoSlot (Variables|Equipment|GetEquipmentSystemSaveObject) (Variables|Equipment|GetEquipmentSystemSlotName))
  (return))

(fn LoadContainer
  (params (SaveName :type String))
  (bind _savedcontainers (Variables|Inventory|GetSavedContainers))
  (bind (_value _returnvalue) (Utilities|Map|Find _savedcontainers SaveName))
  (return _returnvalue _value))

(fn LoadEquipment
  (params (SaveName :type String))
  (bind _savedequipment (Variables|Equipment|GetSavedEquipment))
  (bind (_value _returnvalue) (Utilities|Map|Find _savedequipment SaveName))
  (return _returnvalue _value))

(fn LoadPlayerInventoryData
  (params (SaveName :type String))
  (bind _savedplayerdata (Variables|Inventory|GetSavedPlayerData))
  (bind (_value _returnvalue) (Utilities|Map|Find _savedplayerdata SaveName))
  (return _returnvalue _value))