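; BP_DemoQuestNPC is a demo quest NPC that makes itself known to players who come within its two overlap ranges.
; StateRefreshRange registers and unregisters the NPC's BPCQuestNPC component with the overlapping actor's BPC_PlayerQuestManager, so its quest state updates while nearby.
; InteractRange adds and removes the NPC in BP_DemoCharacter's InteractionRangeNPCs array, tracking which NPCs are within interaction range.
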(event OnComponentBeginOverlap(StateRefreshRange)
  (params (OverlappedComponent :type Primitive%20Component%20Object%20Reference) (OtherActor :type Actor%20Object%20Reference) (OtherComp :type Primitive%20Component%20Object%20Reference) (OtherBodyIndex :type Integer) (bFromSweep :type Boolean) (SweepResult :type Hit%20Result%20Structure%20%28by%20ref%29))
  (bind _returnvalue (Actor|GetComponentbyClass OtherActor "/Game/OpenRPG_Quests/Blueprints/Components/BPC_PlayerQuestManager.BPC_PlayerQuestManager_C"))
  ;[0.1042 0.1042 0.1042] Register or unregister to update the state when player enters the refresh sphere
  (Utilities|IsValid _returnvalue
    (:Is%20Valid
      (Default|RegisterNearbyNPC _returnvalue (Variables|Default|GetBPC_QuestNPC)))))

(event OnComponentEndOverlap(StateRefreshRange)
  (params (OverlappedComponent :type Primitive%20Component%20Object%20Reference) (OtherActor :type Actor%20Object%20Reference) (OtherComp :type Primitive%20Component%20Object%20Reference) (OtherBodyIndex :type Integer))
  (bind _returnvalue (Actor|GetComponentbyClass OtherActor "/Game/OpenRPG_Quests/Blueprints/Components/BPC_PlayerQuestManager.BPC_PlayerQuestManager_C"))
  ;[0.1042 0.1042 0.1042] Register or unregister to update the state when player enters the refresh sphere
  (Utilities|IsValid _returnvalue
    (:Is%20Valid
      (Default|UnregisterNearbyNPC _returnvalue (Variables|Default|GetBPC_QuestNPC)))))

(event OnComponentBeginOverlap(InteractRange)
  (params (OverlappedComponent :type Primitive%20Component%20Object%20Reference) (OtherActor :type Actor%20Object%20Reference) (OtherComp :type Primitive%20Component%20Object%20Reference) (OtherBodyIndex :type Integer) (bFromSweep :type Boolean) (SweepResult :type Hit%20Result%20Structure%20%28by%20ref%29))
  ;[0.05208 0.05208 0.05208] Register or unregister this NPC in the player array
  (bind _asbp_demo_character (Utilities|Casting|CastToBP_DemoCharacter OtherActor))
  (Utilities|Array|Add (Variables|/Game/Quest_Demo/Blueprints/BP_DemoCharacter.BP_DemoCharacter_C|GetInteractionRangeNPCs _asbp_demo_character) self))

(event OnComponentEndOverlap(InteractRange)
  (params (OverlappedComponent :type Primitive%20Component%20Object%20Reference) (OtherActor :type Actor%20Object%20Reference) (OtherComp :type Primitive%20Component%20Object%20Reference) (OtherBodyIndex :type Integer))
  ;[0.05208 0.05208 0.05208] Register or unregister this NPC in the player array
  (bind _asbp_demo_character (Utilities|Casting|CastToBP_DemoCharacter OtherActor))
  (Utilities|Array|RemoveItem (Variables|/Game/Quest_Demo/Blueprints/BP_DemoCharacter.BP_DemoCharacter_C|GetInteractionRangeNPCs _asbp_demo_character) self))

(fn ConstructionScript)